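; BP_Character is the player character for a two-player bomb-dropping game, with world-axis movement and tintable material.
; Player 1 input drives this pawn directly, while Player 2 input is forwarded to the pawn of player controller 1.
; DropBomb spawns a BP_Bomb snapped to a 100-unit grid while under the bomb limit, passing its explosion length.
; Power-up functions raise explosion length, bomb limit and walk speed, and OnBombDestroyed frees a bomb slot.
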(event EventBeginPlay)

(event Collision|EventActorBeginOverlap
  (params (OtherActor :type Actor%20Object%20Reference)))

(event EventTick
  (params (DeltaSeconds :type Float%20%28single-precision%29)))

(event Input|ActionEvents|InputActionPlayer1DropBomb
  (params (Key :type Key%20Structure))
  ;[1 1 1] Player 1 Control
  (:Pressed
    (CallFunction|DropBomb)))

(event Input|ActionEvents|InputActionPlayer2DropBomb
  (params (Key :type Key%20Structure))
  ;[1 1 1] Player 2 Control
  (:Pressed
    (bind _asbp_character (Utilities|Casting|CastToBP_Character (Pawn|GetControlledPawn (Game|GetPlayerController 1))))
    (CallFunction|DropBomb _asbp_character)))

(event Input|AxisEvents|InputAxisPlayer2Up
  (params (AxisValue :type Float%20%28single-precision%29))
  ;[1 1 1] Player 2 Control
  (bind _asbp_character (Utilities|Casting|CastToBP_Character (Pawn|GetControlledPawn (Game|GetPlayerController 1))))
  (Pawn|Input|AddMovementInput _asbp_character "1.000000, 0, 0" AxisValue true))

(event Input|AxisEvents|InputAxisPlayer2Right
  (params (AxisValue :type Float%20%28single-precision%29))
  ;[1 1 1] Player 2 Control
  (bind _asbp_character (Utilities|Casting|CastToBP_Character (Pawn|GetControlledPawn (Game|GetPlayerController 1))))
  (Pawn|Input|AddMovementInput _asbp_character "0.000000,1.000000, 0" AxisValue true))

(event Input|AxisEvents|InputAxisPlayer1Right
  (params (AxisValue :type Float%20%28single-precision%29))
  ;[1 1 1] Player 1 Control
  (Pawn|Input|AddMovementInput "0,1.000000, 0" AxisValue true))

(event Input|AxisEvents|InputAxisPlayer1Up
  (params (AxisValue :type Float%20%28single-precision%29))
  ;[1 1 1] Player 1 Control
  (Pawn|Input|AddMovementInput "1.000000, 0, 0" AxisValue true))

(fn ConstructionScript)

(fn RoundtoNearest
  (params (Value :type Float%20%28single-precision%29) (Multiple :type Float%20%28single-precision%29))
  (return (* (Math|Float|Round (/ (+ Value 0.5) Multiple)) Multiple)))

(fn ExplosionPowerUp
  (Variables|Default|SetExplosionLength (+ (Variables|Default|GetExplosionLength) 1e+02)))

(fn BombPowerUp
  (Math|Integer|IncrementInt (Variables|Default|GetMaxBombs)))

(fn SpeedPowerUp
  (bind _charactermovement (Variables|Character|GetCharacterMovement))
  (Variables|/Script/Engine.CharacterMovementComponent|SetMaxWalkSpeed _charactermovement (+ (Variables|/Script/Engine.CharacterMovementComponent|GetMaxWalkSpeed _charactermovement) 5e+01)))

(fn OnBombDestroyed
  (Math|Integer|DecrementInt (Variables|Default|GetNumBombs)))

(fn SetColour
  (params (Colour :type Linear%20Color%20Structure))
  (bind _returnvalue (Rendering|Material|CreateDynamicMaterialInstance (Variables|Character|GetMesh) 0 0 :!class /Script/Engine.PrimitiveComponent))
  (Rendering|Material|SetVectorParameterValue _returnvalue "BaseColor" Colour :!class /Script/Engine.MaterialInstanceDynamic))

(fn DropBomb
  (bind _returnvalue (Transformation|GetActorTransform))
  (bind (_x _y) (Math|Vector|BreakVector (.location _returnvalue)))
  (Math|Integer|CompareInt (Variables|Default|GetNumBombs) (Variables|Default|GetMaxBombs)
    (:<
      (Game|SpawnActorfromClass "/Game/Blueprints/BP_Bomb.BP_Bomb_C" (Math|Transform|MakeTransform (Math|Vector|MakeVector (CallFunction|RoundtoNearest _x 1e+02) (CallFunction|RoundtoNearest _y 1e+02) 55.0) "0, 0, 0" "1,1,1") "AlwaysSpawn" self (Variables|Default|GetExplosionLength) 0)
      (Math|Integer|IncrementInt (Variables|Default|GetNumBombs)))))