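; BP_ExplosionLine is an actor that acts as one growing arm of an explosion, traveling along its forward vector.
; Each Tick extends its length up to a maximum and line traces on the Camera channel from slightly above its origin, with debug drawing on.
; On a hit it destroys itself, destroys any BP_BreakableCube struck and calls SpawnExplosion on any BP_Bomb.
; Without a hit, it destroys itself upon reaching maximum length.
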(event EventBeginPlay)

(event Collision|EventActorBeginOverlap
  (params (OtherActor :type Actor%20Object%20Reference)))

(event EventTick
  (params (DeltaSeconds :type Float%20%28single-precision%29))
  (bind _returnvalue (Transformation|GetActorLocation))
  (bind _returnvalue_2 (+ _returnvalue "0, 0,50.000000"))
  (Variables|Default|SetCurLength (Math|Float|Clamp(Float) (+ (* (Variables|Default|GetLengthRate) DeltaSeconds) (Variables|Default|GetCurLength)) 0.0 (Variables|Default|GetMaxLength)))
  (bind (_outhit _returnvalue_3) (Collision|LineTraceByChannel _returnvalue_2 (+ _returnvalue_2 (* (Math|Vector|GetForwardVector (Transformation|GetActorRotation)) (Math|Float|Clamp(Float) (+ (* (Variables|Default|GetLengthRate) DeltaSeconds) (Variables|Default|GetCurLength)) 0.0 (Variables|Default|GetMaxLength)))) "TraceTypeQuery2" false 0 "ForDuration" true "(R=1.000000,G=0.000000,B=0.000000,A=1.000000)" "(R=0.000000,G=1.000000,B=0.000000,A=1.000000)" 1.0))
  (if _returnvalue_3
    (Actor|DestroyActor)
    (Utilities|FlowControl|Sequence
      (:then_0
        (bind _asbp_breakable_cube (Utilities|Casting|CastToBP_BreakableCube (.HitActor (Collision|BreakHitResult _outhit))))
        (Actor|DestroyActor _asbp_breakable_cube))
      (:then_1
        (bind _asbp_bomb (Utilities|Casting|CastToBP_Bomb (.HitActor (Collision|BreakHitResult _outhit))))
        (Default|SpawnExplosion _asbp_bomb "0, 0, 0")))
    (elif (Math|Float|NearlyEqual(Float) (Variables|Default|GetCurLength) (Variables|Default|GetMaxLength) 0.001)
      (Actor|DestroyActor))))

(fn ConstructionScript)