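; BP_BreakableCube is a breakable cube actor that can drop a random power-up when destroyed.
; Its Destroyed event rolls a roughly even chance to call SpawnPowerUp, then calls DestroyActor on itself regardless of the result.
; SpawnPowerUp picks a random class from the PowerUps array and always spawns it slightly above the cube's location, ignoring collisions.
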(event EventBeginPlay)

(event EventEndPlay
  (params (EndPlayReason :type EEndPlayReason%20Enum :default "Destroyed")))

(event EventTick
  (params (DeltaSeconds :type Float%20%28single-precision%29)))

(event EventDestroyed
  (Utilities|FlowControl|Sequence
    (:then_0
      (if (<= (Math|Random|RandomFloat) 0.5)
        (CallFunction|SpawnPowerUp)))
    (:then_1
      (Actor|DestroyActor))))

(fn ConstructionScript)

(fn SpawnPowerUp
  (bind _returnvalue (Transformation|GetActorLocation))
  (Game|SpawnActorfromClass (Utilities|Array|Get(acopy) (Variables|Default|GetPowerUps) (Math|Random|RandomIntegerinRange 0 (- (Utilities|Array|Length (Variables|Default|GetPowerUps)) 1))) (Math|Transform|MakeTransform (Math|Vector|MakeVector (.x _returnvalue) (.y _returnvalue) (+ (.z _returnvalue) 5e+01)) "0, 0, 0" "1,1,1") "AlwaysSpawn" 0 0))