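; Level actor that scatters breakable cubes over a Bomberman-style grid at BeginPlay, after destroying any existing ones.
; It builds candidate cells on a fixed world-space grid, skipping odd/odd cells and points inside BlockingVolume bounds.
; A Density fraction sets the number of random draws; picks too close to recorded cubes are skipped.
; RandomLocation rolls separate indices for reading and removing, both with an upper bound of array length.
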(event Custom|PlaceBlocks
  (CallFunction|PopulateValidLocations)
  (CallFunction|ClearBlocks)
  (bind _output_get (Variables|Default|SetNumberOfBlocks (Math|Float|Truncate (* (Utilities|Array|Length (Variables|Default|GetValidLocations)) (Variables|Default|GetDensity)))))
  (for _index (range 1 _output_get)
    (bind (_location _valid) (CallFunction|RandomLocation))
    (if _valid
      (bind _returnvalue (Game|SpawnActorfromClass "/Game/Blueprints/BP_BreakableCube.BP_BreakableCube_C" (Math|Transform|MakeTransform (Math|Vector|MakeVector (.x _location) (.y _location) 5e+01) "0, 0, 0" "1,1,1") "AlwaysSpawn" 0 0))
      (Utilities|Array|Add (Variables|Default|GetSelectedLocation) (Transformation|GetActorLocation _returnvalue)))))

(event Custom|PopulateValidLocations
  (Utilities|Array|Clear (Variables|Default|GetValidLocations))
  (for _index (range 0 10)
    (for _index_2 (range 0 12)
      (if (not (and (== (Math|Integer|%(Integer) _index_2 2) 1) (== (Math|Integer|%(Integer) _index 2) 1)))
        (bind _valid (CallFunction|IsPointValid (Math|Vector|MakeVector (* _index 1e+02) (* _index_2 1e+02) 5e+01)))
        (if _valid
          (Utilities|Array|Add (Variables|Default|GetValidLocations) (Math|Vector|MakeVector (* _index 1e+02) (* _index_2 1e+02) 5e+01)))))))

(event Custom|ClearBlocks
  (bind _outactors (Actor|GetAllActorsOfClass "/Game/Blueprints/BP_BreakableCube.BP_BreakableCube_C"))
  (for _array_element _outactors
    (Actor|DestroyActor _array_element)))

(event EventBeginPlay
  (CallFunction|PlaceBlocks))

(event Collision|EventActorBeginOverlap
  (params (OtherActor :type Actor%20Object%20Reference)))

(event EventTick
  (params (DeltaSeconds :type Float%20%28single-precision%29)))

(fn ConstructionScript)

(fn RandomLocation
  (bind _validlocations (Variables|Default|GetValidLocations))
  (bind _validlocations_2 (Variables|Default|GetValidLocations))
  (bind _returnvalue (Utilities|Array|Length _validlocations))
  (bind _returnvalue_2 (Math|Random|RandomIntegerinRange 0 _returnvalue))
  (bind _output_get (LocalVariables|SetRandLocation (Utilities|Array|Get(acopy) _validlocations_2 _returnvalue_2)))
  (Utilities|Array|RemoveIndex _validlocations_2 _returnvalue_2)
  (for _array_element (Variables|Default|GetSelectedLocation)
    (if (< (Math|Vector|VectorLength (- _output_get _array_element)) 1e+02)
      (return "0, 0, 0" false)))
  (return _output_get true))

(fn IsPointValid
  (params (Vector :type Vector))
  (bind _outactors (Actor|GetAllActorsOfClass "/Script/Engine.BlockingVolume"))
  (for _array_element _outactors
    (if (Math|Geometry|IsPointinBox Vector (.Origin (Collision|GetActorBounds _array_element false)) (.BoxExtent (Collision|GetActorBounds _array_element false)))
      (return false)))
  (for _array_element_2 (Variables|Default|GetSelectedLocation)
    (if (< (Math|Vector|VectorLength (- Vector _array_element_2)) 1e+02)
      (Development|PrintString "Duplicate")
      (return false)))
  (return true))